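; FPS grappling hook actor that, on hit, hands the grapple off to the player's FPS_Character.
; It records the character's location as the grapple start and the hit location as the end.
; If no hook is already connected, it triggers the character's MoveGrapple and GrappleLanded.
; It then polls IsGrappling through a near-zero Delay loop and destroys itself once grappling ends.
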(event EventBeginPlay)

(event Collision|EventActorBeginOverlap
  (params (OtherActor :type Actor%20Object%20Reference)))

(event EventTick
  (params (DeltaSeconds :type Float%20%28single-precision%29)))

(event Collision|EventHit
  (params (MyComp :type Primitive%20Component%20Object%20Reference) (Other :type Actor%20Object%20Reference) (OtherComp :type Primitive%20Component%20Object%20Reference) (bSelfMoved :type Boolean) (HitLocation :type Vector :default "0, 0, 0") (HitNormal :type Vector :default "0, 0, 0") (NormalImpulse :type Vector :default "0, 0, 0") (Hit :type Hit%20Result%20Structure%20%28by%20ref%29))
  (bind _asfps_character (Utilities|Casting|CastToFPS_Character (Game|GetPlayerCharacter 0)))
  (Variables|/Game/BLUEPRINTS/Player/FPS_Character.FPS_Character_C|SetGrappleStartLocation _asfps_character (Transformation|GetActorLocation _asfps_character))
  (Variables|/Game/BLUEPRINTS/Player/FPS_Character.FPS_Character_C|SetGrappleEndLocation _asfps_character HitLocation)
  (if (not (Variables|/Game/BLUEPRINTS/Player/FPS_Character.FPS_Character_C|GetbHookConnected _asfps_character))
    (Default|MoveGrapple _asfps_character)
    (Default|GrappleLanded _asfps_character)
    (Utilities|FlowControl|Delay 0.0001 :!label _label)
    (if (not (Variables|/Game/BLUEPRINTS/Player/FPS_Character.FPS_Character_C|GetbIsGrappling _asfps_character))
      (Actor|DestroyActor)
      (Variables|/Game/BLUEPRINTS/Player/FPS_Character.FPS_Character_C|SetbIsGrappling _asfps_character false)
      (else
        (goto _label)))))

(fn ConstructionScript)