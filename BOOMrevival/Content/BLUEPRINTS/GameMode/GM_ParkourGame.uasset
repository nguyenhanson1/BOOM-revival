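; Parkour game mode that sets initial spawn points for FPS_Character players and handles their respawning.
; One second after BeginPlay, it gives every existing character the StartSpawn transform.
; Respawn spawns a new character at the old one's stored transform, copies that transform and Score, then has the controller possess it.
; The old pawn is not destroyed here, and both events print character names for debugging.
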(event Custom|Respawn
  (params (FPSCharacter :type FPS%20Character%20Object%20Reference))
  (Development|PrintString (Utilities|String|Append (Utilities|GetDisplayName FPSCharacter) ""))
  (bind _returnvalue (Game|SpawnActorfromClass "/Game/BLUEPRINTS/Player/FPS_Character.FPS_Character_C" (Variables|/Game/BLUEPRINTS/Player/FPS_Character.FPS_Character_C|GetSpawnTransform FPSCharacter) "AdjustIfPossibleButAlwaysSpawn" 0 0))
  (Variables|/Game/BLUEPRINTS/Player/FPS_Character.FPS_Character_C|SetSpawnTransform _returnvalue (Variables|/Game/BLUEPRINTS/Player/FPS_Character.FPS_Character_C|GetSpawnTransform FPSCharacter))
  (Variables|/Game/BLUEPRINTS/Player/FPS_Character.FPS_Character_C|SetScore _returnvalue (Variables|/Game/BLUEPRINTS/Player/FPS_Character.FPS_Character_C|GetScore FPSCharacter))
  (Pawn|Possess (Pawn|GetController FPSCharacter) _returnvalue))

(event EventBeginPlay
  (Utilities|FlowControl|Delay 1.0)
  (bind _outactors (Actor|GetAllActorsOfClass "/Game/BLUEPRINTS/Player/FPS_Character.FPS_Character_C"))
  (for _array_element _outactors
    (Development|PrintString (Utilities|GetDisplayName _array_element))
    (Variables|/Game/BLUEPRINTS/Player/FPS_Character.FPS_Character_C|SetSpawnTransform _array_element (Variables|Default|GetStartSpawn))))

(fn ConstructionScript)