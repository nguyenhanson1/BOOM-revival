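; ScoreTarget is a parkour game target that awards points when a player damages it.
; On any damage instigated by a PlayerController, it adds ScoreValue to GM_ParkourGame's score and destroys itself.
; The construction script shows ScoreValue on a text render and scales the sphere by SphereScale.
; Each tick it rotates the text to face the player camera.
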(event EventBeginPlay)

(event Collision|EventActorBeginOverlap
  (params (OtherActor :type Actor%20Object%20Reference)))

(event EventTick
  (params (DeltaSeconds :type Float%20%28single-precision%29))
  (Transformation|SetWorldRotation (Variables|Default|GetTextRender) (Math|Rotator|MakeRotfromX (- (Transformation|GetActorLocation (Game|GetPlayerCameraManager 0)) (Transformation|GetWorldLocation (Variables|Default|GetTextRender)))) false false))

(event Game|Damage|EventAnyDamage
  (params (Damage :type Float%20%28single-precision%29) (DamageType :type Damage%20Type%20Object%20Reference) (InstigatedBy :type Controller%20Object%20Reference) (DamageCauser :type Actor%20Object%20Reference))
  (Utilities|Casting|CastToPlayerController InstigatedBy)
  (bind _asgm_parkour_game (Utilities|Casting|CastToGM_ParkourGame (Game|GetGameMode)))
  (Default|AddScore _asgm_parkour_game (Variables|Score|GetscoreValue))
  (Actor|DestroyActor))

(fn ConstructionScript
  (Rendering|Components|TextRender|SetText (Variables|Default|GetTextRender) (Utilities|Text|ToText(Integer) (Variables|Score|GetscoreValue)))
  (Transformation|SetRelativeScale3D (Variables|Default|GetSphere) (* "1.000000,1.000000,1.000000" (Variables|Score|GetsphereScale))))