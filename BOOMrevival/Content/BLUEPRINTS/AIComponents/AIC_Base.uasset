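; Base AI controller that runs the melee behavior tree and blackboard, turning perception stimuli into AI states.
; Sight of a player-team actor triggers attacking, seeking when lost, or passive if dead; gunshots trigger seeking and other noises investigating, at navmesh-projected points.
; State setters write blackboard keys and notify the pawn by interface message.
; Once attacking, it ignores further sight and hearing stimuli; damage processing is an empty stub.
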(event OnPerceptionUpdated(AIPerception)
  (params (UpdatedActors :type Array%20of%20Actor%20Object%20References))
  (for _array_element UpdatedActors
    (bind _info (Class|AIPerceptionComponent|GetActorsPerception (Variables|Default|GetAIPerception) _array_element))
    (Variables|Default|SetActorSensed (.target _info))
    (for _array_element_2 (.lastsensedstimuli _info)
      (bind _output_get (Variables|Default|SetActorSensedStimuli _array_element_2))
      (bind _returnvalue (Class|AIPerceptionSystem|GetSenseClassforStimulus _output_get))
      (if (== _returnvalue "/Script/AIModule.AISense_Sight")
        (CallFunction|ProcessSightStimuli)
        (elif (== _returnvalue "/Script/AIModule.AISense_Hearing")
          (CallFunction|ProcessHearingStimuli))))))

(event EventBeginPlay
  (Class|AIController|UseBlackboard "/Game/BLUEPRINTS/AIComponents/BB_Melee.BB_Melee")
  (AI|RunBehaviorTree "/Game/BLUEPRINTS/AIComponents/BT_Melee.BT_Melee")
  (AI|Components|Blackboard|SetValueasVector (Variables|Default|GetBlackboard) (Utilities|Name|MakeLiteralName "SpawnLocation") (Transformation|GetActorLocation (Pawn|GetControlledPawn))))

(event EventTick
  (params (DeltaSeconds :type Float%20%28single-precision%29)))

(fn ConstructionScript)

(fn ProcessSightStimuli
  (bind _actorsensedstimuli (Variables|Default|GetActorSensedStimuli))
  (bind _actorsensed (Variables|Default|GetActorSensed))
  (bind (_age _expirationage _strength _stimuluslocation _receiverlocation _tag _bsuccessfullysensed) (Utilities|Struct|BreakAIStimulus _actorsensedstimuli))
  ;[1 1 1] Check if AI seen player
  (if (Utilities|DoesObjectImplementInterface _actorsensed "/Game/BLUEPRINTS/Interface/BPI_AI.BPI_AI_C")
    (bind _isplayer (Class|BPIAI|GetTeamID(Message) _actorsensed))
    (if (and _isplayer (CallFunction|IsNotAttacking))
      ;[1 1 1] Detected Actor is the player
      (bind _isdead (Class|BPIAI|IsDead(Message) (Variables|Default|GetActorSensed)))
      (if _isdead
        (States|SetStatesasPassive)
        (elif _bsuccessfullysensed
          (States|SetStateasAttacking (Variables|Default|GetActorSensed))
          (else
            (States|SetStateasSeeking _stimuluslocation)))))))

(fn ProcessHearingStimuli
  (bind _actorsensedstimuli (Variables|Default|GetActorSensedStimuli))
  (bind (_age _expirationage _strength _stimuluslocation _receiverlocation _tag _bsuccessfullysensed) (Utilities|Struct|BreakAIStimulus _actorsensedstimuli))
  (bind _projectedlocation (AI|Navigation|ProjectPointtoNavigation _stimuluslocation 0 0 "500.000000,500.000000,200.000000"))
  (if (and (CallFunction|IsNotAttacking) _bsuccessfullysensed)
    (if (Utilities|Name|Equal(Name) _tag "GunShot")
      (States|SetStateasSeeking _projectedlocation)
      (else
        (States|SetStateasInvestigating _projectedlocation _stimuluslocation)))))

(fn ProcessDamageStimuli
  (if (and (CallFunction|IsNotAttacking) (.bSuccessfullySensed (Utilities|Struct|BreakAIStimulus (Variables|Default|GetActorSensedStimuli))))
    _))

(fn IsNotAttacking
  (return (Utilities|Enum|NotEqual(Enum) (Utilities|Enum|ByteToEnumAIStates (Class|BlackboardComponent|GetValueasEnum (AI|GetBlackboard 0) (Variables|KeyName|GetStateKey))) "NewEnumerator3")))

(fn SetStatesasPassive
  (bind _returnvalue (Utilities|Enum|LiteralenumAIStates "NewEnumerator0"))
  (AI|Components|Blackboard|SetValueasEnum (Variables|Default|GetBlackboard) (Variables|KeyName|GetStateKey) _returnvalue)
  (AI|Components|Blackboard|SetValueasBool (Variables|Default|GetBlackboard) (Variables|KeyName|GetHasLOSKey) false)
  (Class|BPIAI|NotifyStateChange(Message) (Pawn|GetControlledPawn) _returnvalue))

(fn SetStateasAttacking
  (params (Target :type Actor%20Object%20Reference))
  (bind _returnvalue (Utilities|Enum|LiteralenumAIStates "NewEnumerator3"))
  (AI|Components|Blackboard|SetValueasEnum (Variables|Default|GetBlackboard) (Variables|KeyName|GetStateKey) _returnvalue)
  (AI|Components|Blackboard|SetValueasObject (Variables|Default|GetBlackboard) (Variables|KeyName|GetTargetKey) Target)
  (AI|Components|Blackboard|SetValueasBool (Variables|Default|GetBlackboard) (Variables|KeyName|GetHasLOSKey) true)
  (Class|BPIAI|NotifyStateChange(Message) (Pawn|GetControlledPawn) _returnvalue))

(fn SetStateasSeeking
  (params (Search :type Vector))
  (bind _returnvalue (Utilities|Enum|LiteralenumAIStates "NewEnumerator2"))
  (AI|Components|Blackboard|SetValueasEnum (Variables|Default|GetBlackboard) (Variables|KeyName|GetStateKey) _returnvalue)
  (AI|Components|Blackboard|SetValueasVector (Variables|Default|GetBlackboard) (Variables|KeyName|GetMoveToKey) Search)
  (Class|BPIAI|NotifyStateChange(Message) (Pawn|GetControlledPawn) _returnvalue))

(fn SetStateasInvestigating
  (params (MoveToLocation :type Vector) (PointOfInterest :type Vector))
  (bind _returnvalue (Utilities|Enum|LiteralenumAIStates "NewEnumerator1"))
  (AI|Components|Blackboard|SetValueasEnum (Variables|Default|GetBlackboard) (Variables|KeyName|GetStateKey) _returnvalue)
  (AI|Components|Blackboard|SetValueasVector (Variables|Default|GetBlackboard) (Variables|KeyName|GetMoveToKey) MoveToLocation)
  (AI|Components|Blackboard|SetValueasVector (Variables|Default|GetBlackboard) (Variables|KeyName|GetPointOfInterest) PointOfInterest)
  (Class|BPIAI|NotifyStateChange(Message) (Pawn|GetControlledPawn) _returnvalue))

(fn SetStateasDead
  (bind _returnvalue (Utilities|Enum|LiteralenumAIStates "NewEnumerator4"))
  (AI|Components|Blackboard|SetValueasEnum (Variables|Default|GetBlackboard) (Variables|KeyName|GetStateKey) _returnvalue)
  (Class|BPIAI|NotifyStateChange(Message) (Pawn|GetControlledPawn) _returnvalue))