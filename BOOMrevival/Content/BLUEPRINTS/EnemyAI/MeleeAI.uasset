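; Melee enemy AI character Blueprint that handles its own death and exposes attack range, team and alive-state queries.
; On the health component's death event, it fires once to turn the mesh into a simulated ragdoll, disable capsule collision and stop the AI controller's brain logic.
; State changes are forwarded to the anim instance, while the team ID and dead queries return fixed defaults and damage events are unhandled.
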(event OnDamageTaken(AC_HealthComponent))

(event OnDeath(AC_HealthComponent)
  (bind _self self)
  (bind _returnvalue (Utilities|GetDisplayName _self))
  (bind _returnvalue_2 (Utilities|String|Append _returnvalue " Died"))
  (Utilities|FlowControl|DoOnce false
    (:Completed
      (Collision|SetCollisionProfileName (Variables|Character|GetMesh) "Ragdoll" true :!class /Script/Engine.PrimitiveComponent)
      (Class|SkeletalMeshComponent|SetAllBodiesSimulatePhysics (Variables|Character|GetMesh) true)
      (Class|PrimitiveComponent|WakeAllRigidBodies (Variables|Character|GetMesh))
      (Collision|SetCollisionEnabled (Variables|Collision|GetCapsuleComponent) "NoCollision")
      (Development|PrintString _returnvalue_2)
      (AI|Logic|StopLogic (Variables|/Script/AIModule.AIController|GetBrainComponent (AI|GetAIController self)) _returnvalue_2))))

(event EventBeginPlay)

(event Collision|EventActorBeginOverlap
  (params (OtherActor :type Actor%20Object%20Reference)))

(event EventTick
  (params (DeltaSeconds :type Float%20%28single-precision%29)))

(event EventNotifyStateChange
  (params (NewState :type AIStates%20Enum :default "NewEnumerator0"))
  (Class|BPIAI|NotifyStateChange(Message) (Components|SkeletalMesh|GetAnimInstance (Variables|Character|GetMesh)) NewState))

(fn ConstructionScript)

(fn GetAttackRange
  (return (Variables|Default|GetAttackRange)))

(fn GetTeamID
  (return false))

(fn IsDead
  (return false))