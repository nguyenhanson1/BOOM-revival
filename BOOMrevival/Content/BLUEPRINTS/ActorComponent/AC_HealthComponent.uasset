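; AC_HealthComponent is an actor component that tracks health for the actor it is attached to.
; On BeginPlay it fills Health from MaxHealth and binds TakeDamage to the owner's OnTakeAnyDamage event.
; Positive damage fires the OnDamageTaken dispatcher, lowers Health and prints the new value, then fires OnDeath if health is zero or below.
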(event Custom|TakeDamage
  (params (DamagedActor :type Actor%20Object%20Reference) (Damage :type Float%20%28single-precision%29) (DamageType :type Damage%20Type%20Object%20Reference) (InstigatedBy :type Controller%20Object%20Reference) (DamageCauser :type Actor%20Object%20Reference))
  ;[1 1 1] Call Damage Taken and Reduce Health
  (if (> Damage 0.0)
    (Default|CallOnDamageTaken)
    (bind _output_get (Variables|Default|SetHealth (- (Variables|Default|GetHealth) Damage)))
    (Development|PrintString (Utilities|String|ToString(Float) _output_get))
    ;[1 1 1] Call OnDeath observers
    (if (CallFunction|IsDead)
      (Default|CallOnDeath))))

(event EventBeginPlay
  (Variables|Default|SetHealth (Variables|Default|GetMaxHealth))
  (EventDispatchers|AssignOnTakeAnyDamage (Components|GetOwner) (delegate Custom|TakeDamage)))

(event EventTick
  (params (DeltaSeconds :type Float%20%28single-precision%29)))

(fn IsDead
  (return (<= (Variables|Default|GetHealth) 0.0)))